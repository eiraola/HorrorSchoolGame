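; A corridor door actor for the horror school game that slides between open and closed positions when its CloseDoor or OpenDoor events are called.
; CloseDoor enables collision, plays a sound and runs a timeline that lerps the mesh's world location between begin and end gizmo components.
; OpenDoor disables collision, plays the sound and reverses the same timeline from its end.
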(event EventBeginPlay)

(event Collision|EventActorBeginOverlap
  (params (OtherActor :type Actor%20Object%20Reference)))

(event EventTick
  (params (DeltaSeconds :type Float%20%28single-precision%29)))

(event EventCloseDoor
  (Class|DoorActor|EnableDoorCollisions)
  (Class|DoorActor|PlayDoorSound)
  (bind _doormovement (Timeline|Door_Movement PlayFromStart)
    (:Update
      (Transformation|SetWorldLocation (Variables|Default|GetDoorStaticMesh) (Math|Vector|Lerp(Vector) (Transformation|GetWorldLocation (Variables|Default|GetDoorBeginPositionGizmo)) (Transformation|GetWorldLocation (Variables|Default|GetDoorEndPositionGizmo)) _doormovement) false false))))

(event EventOpenDoor
  (Class|DoorActor|DisableDoorCollisions)
  (Class|DoorActor|PlayDoorSound)
  (bind _doormovement (Timeline|Door_Movement ReverseFromEnd)
    (:Update
      (Transformation|SetWorldLocation (Variables|Default|GetDoorStaticMesh) (Math|Vector|Lerp(Vector) (Transformation|GetWorldLocation (Variables|Default|GetDoorBeginPositionGizmo)) (Transformation|GetWorldLocation (Variables|Default|GetDoorEndPositionGizmo)) _doormovement) false false))))

(fn ConstructionScript)